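; Ball launcher actor that automatically fires small balls, each carrying a grenade modifier.
; A looping timer started on BeginPlay spawns a scaled-down Ball at the Spawn component every two seconds.
; Each ball's ProjectileMovement gets a fixed-speed velocity in a random direction within a cone around the Arrow's forward vector.
; A grenade modifier actor is then spawned, attached to the ball and flagged ReadyToThrow.
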(event Custom|FIre
  (bind _spawn (Variables|Default|GetSpawn))
  (bind _returnvalue (Game|SpawnActorfromClass "/Game/CustomMaps/UGC2078691775/blueprints/grenade_stuff/ball.ball_C" (Math|Transform|MakeTransform (Transformation|GetWorldLocation _spawn) (Transformation|GetWorldRotation _spawn) "0.300000,0.300000,0.300000") "Undefined" 0 0))
  (Variables|/Script/Engine.MovementComponent|SetVelocity (Variables|/Game/CustomMaps/UGC2078691775/blueprints/grenade_stuff/ball.ball_C|GetProjectileMovement _returnvalue) (* (Math|Random|RandomUnitVectorinConeinDegrees (Math|Vector|GetForwardVector (Variables|Default|GetArrow)) 3e+01) 2e+03))
  (bind _returnvalue_2 (Game|SpawnActorfromClass "/Game/CustomMaps/UGC2078691775/blueprints/modifiers/grenade_modifier.grenade_modifier_C" (Math|Transform|MakeTransform "0, 0, 0") "Undefined" 0 0))
  (Transformation|AttachActorToActor _returnvalue_2 _returnvalue "None" "KeepRelative" "KeepRelative" "KeepRelative" true)
  (Variables|/Game/CustomMaps/UGC2078691775/blueprints/modifiers/grenade_modifier.grenade_modifier_C|SetreadyToThrow _returnvalue_2 true))

(event EventBeginPlay
  (Utilities|Time|SetTimerbyEvent (delegate Custom|FIre) 2.0 true))

(fn ConstructionScript)