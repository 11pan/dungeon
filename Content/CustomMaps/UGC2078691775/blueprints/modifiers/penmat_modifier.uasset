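; Map modifier that swaps one material slot on a target to a penetrable material while the modifier exists.
; BeginPlay caches the material at the configured index, then applies the replacement.
; EndPlay restores the cached material only when the modifier is destroyed, not for other end-play reasons.
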(event EventBeginPlay
  (Variables|Default|SetoldMat (Rendering|Material|GetMaterial (Variables|Default|Gettarget) (Variables|Default|GetmatIdx)))
  (Rendering|Material|SetMaterial (Variables|Default|Gettarget) (Variables|Default|GetmatIdx) "/Game/CustomMaps/UGC2078691775/mats/penetrable_mat.penetrable_mat"))

(event EventEndPlay
  (params (EndPlayReason :type EEndPlayReason%20Enum :default "Destroyed"))
  (switch Utilities|FlowControl|Switch|SwitchonEEndPlayReason EndPlayReason
    (:Destroyed
      (Rendering|Material|SetMaterial (Variables|Default|Gettarget) (Variables|Default|GetmatIdx) (Variables|Default|GetoldMat)))))

(fn ConstructionScript)