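; Pavlov custom-map modifier actor that attaches to a grenade and shows a particle trail once it leaves a player's hand or inventory.
; Each tick it switches on the class display name of its grandparent attach actor: controller or inventory turns the trail off and sets ReadyToThrow.
; Any other holder activates the trail if ReadyToThrow is set.
; Without an attach parent, it stops the trail component's tick and destroys itself after a delay.
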(event EventTick
  (params (DeltaSeconds :type Float%20%28single-precision%29))
  (bind _returnvalue (Actor|GetAttachParentActor))
  (bind _trailparticles (Variables|Default|GetTrailParticles))
  (Utilities|IsValid _returnvalue
    (:Is%20Valid
      (switch string (Utilities|GetClassDisplayName (Utilities|GetClass (Actor|GetAttachParentActor _returnvalue)))
        (:Default
          (if (Variables|Default|GetreadyToThrow)
            (Components|Activation|Activate _trailparticles false)))
        (:BP_PavlovController_C
          (Components|Activation|Deactivate _trailparticles :!label _label)
          (Variables|Default|SetreadyToThrow true))
        (:BP_PavlovInventory_C
          (goto _label))))
    (:Is%20Not%20Valid
      (Components|Tick|SetComponentTickEnabled (Variables|Default|GetTrailParticles) false)
      (Utilities|FlowControl|Delay 1e+01)
      (Actor|DestroyActor))))

(fn ConstructionScript)