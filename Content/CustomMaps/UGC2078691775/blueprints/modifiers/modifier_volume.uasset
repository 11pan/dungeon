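; Volume for a Pavlov custom map that attaches modifier actors to the player and to items that enter its box.
; Two seconds after start it modifies the local player, enables box queries and tags existing actors as modified.
; Overlaps are tagged and dispatched by class display name: players, tasers, and knives or grenades, the latter gated by a game-logic setting.
; Bot handling is empty and bullet logic is unconnected.
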(event EventBeginPlay
  (Utilities|FlowControl|Delay 2.0)
  (CallFunction|ModifyPlayer (Game|Player|GetPlayerPawn 0))
  (Collision|SetCollisionEnabled (Variables|Default|GetBox) "QueryOnly")
  (bind _outactors (Actor|GetAllActorsOfClass "/Script/Engine.Actor"))
  (for _array_element _outactors
    (Utilities|AddTag _array_element "modified")))

(event Collision|EventActorBeginOverlap
  (params (OtherActor :type Actor%20Object%20Reference))
  (CallFunction|HandleEntity OtherActor))

(fn ConstructionScript
  (Collision|SetCollisionEnabled (Variables|Default|GetBox) "NoCollision"))

(fn HandleEntity
  (params (Actor :type Actor%20Object%20Reference))
  (bind _output_get (LocalVariables|SetNewEntity Actor))
  (Utilities|AddTag _output_get "modified"
    (:Out
      (switch string (Utilities|GetClassDisplayName (Utilities|GetClass Actor))
        (:Default
          (Utilities|FlowControl|Sequence))
        (:Knife_ST1_C
          (CallFunction|ModifyUtil (LocalVariables|GetNewEntity) :!label _label))
        (:Grenade_Smoke_C
          (goto _label))
        (:Grenade_M64_C
          (goto _label))
        (:Grenade_Flash_c
          (goto _label))
        (:Gun_Taser_C
          (bind _returnvalue (Game|SpawnActorfromClass "/Game/CustomMaps/UGC2078691775/blueprints/modifiers/tool_modifier.tool_modifier_C" (Math|Transform|MakeTransform "0, 0, 0") "Undefined" 0 0))
          (Transformation|AttachActorToActor _returnvalue (LocalVariables|GetNewEntity) "None" "SnapToTarget" "SnapToTarget" "SnapToTarget" true))
        (:BP_PavlovPawn_C
          (bind _aspawn (Utilities|Casting|CastToPawn (LocalVariables|GetNewEntity)))
          (Utilities|IsPlayer (LocalVariables|GetNewEntity)
            (:Player
              (CallFunction|ModifyPlayer _aspawn))
            (:Not%20Player
              (CallFunction|ModifyBot _aspawn))))))))

(fn ModifyPlayer
  (params (player :type Pawn%20Object%20Reference))
  (if (not (Actor|ActorHasTag player "modifier_attached"))
    (bind _returnvalue (Game|SpawnActorfromClass "/Game/CustomMaps/UGC2078691775/blueprints/modifiers/player_modifier.player_modifier_C" (Math|Transform|MakeTransform "0, 0, 0") "Undefined" 0 0))
    (Transformation|AttachActorToActor _returnvalue player "None" "SnapToTarget" "SnapToTarget" "SnapToTarget" true)
    (Utilities|AddTag player "modifier_attached")))

(fn ModifyBot
  (params (bot :type Pawn%20Object%20Reference)))

(fn ModifyUtil
  (params (Util :type Actor%20Object%20Reference))
  (bind _gamelogic (Utilities|GetGameLogic)
    (:ExecOut
      (if (Utilities|GetSetting _gamelogic "NewEnumerator0")
        (bind _returnvalue (Game|SpawnActorfromClass "/Game/CustomMaps/UGC2078691775/blueprints/modifiers/grenade_modifier.grenade_modifier_C" (Math|Transform|MakeTransform "0, 0, 0") "Undefined" 0 0))
        (Transformation|AttachActorToActor _returnvalue Util "None" "SnapToTarget" "SnapToTarget" "SnapToTarget" true)))))